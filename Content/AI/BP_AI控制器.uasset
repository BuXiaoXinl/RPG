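; AI controller for enemies that runs the BT_AI behavior tree and feeds its Blackboard from AI Perception updates.
; The sight handler stores the sensed actor as 目标 (target), clearing it on lost sight or any non-sight stimulus, including hearing.
; The hearing handler writes the stimulus location to 听力位置 (heard location) and turns on the controlled BP_AIEnemy's investigation icon.
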(event OnTargetPerceptionUpdated(AIPerception)
  (params (Actor :type Actor%20Object%20Reference) (Stimulus :type AI%20Stimulus%20Structure))
  (CallFunction|AI视力检测 Actor Stimulus)
  (CallFunction|AI听力检测 Actor Stimulus))

(event EventBeginPlay
  (AI|RunBehaviorTree "/Game/AI/BT_AI.BT_AI"))

(fn ConstructionScript)

(fn AI视力检测
  (params (Actor :type Actor%20Object%20Reference) (AI刺激物 :type AI%20Stimulus%20Structure))
  (bind _returnvalue (Class|AIPerceptionSystem|GetSenseClassforStimulus AI刺激物))
  (if (== _returnvalue "/Script/AIModule.AISense_Sight")
    (if (.bSuccessfullySensed (Utilities|Struct|BreakAIStimulus AI刺激物))
      (AI|Components|Blackboard|SetValueasObject (AI|GetBlackboard 0) (Utilities|Name|MakeLiteralName "目标") Actor)
      (else
        (AI|Components|Blackboard|SetValueasObject (AI|GetBlackboard 0) (Utilities|Name|MakeLiteralName "目标") 0 :!label _label)))
    (else
      (goto _label))))

(fn AI听力检测
  (params (Actor :type Actor%20Object%20Reference) (AI刺激物 :type AI%20Stimulus%20Structure))
  (bind _returnvalue (Class|AIPerceptionSystem|GetSenseClassforStimulus AI刺激物))
  (if (== _returnvalue "/Script/AIModule.AISense_Hearing")
    (AI|Components|Blackboard|SetValueasVector (AI|GetBlackboard 0) (Utilities|Name|MakeLiteralName "听力位置") (.StimulusLocation (Utilities|Struct|BreakAIStimulus AI刺激物)))
    (bind _asbp_aienemy (Utilities|Casting|CastToBP_AIEnemy (Pawn|GetControlledPawn)))
    (Default|启用调查图标 _asbp_aienemy)))