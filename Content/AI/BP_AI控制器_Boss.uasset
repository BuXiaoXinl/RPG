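; Boss AI controller that runs the boss behavior tree and manages the boss fight health bar UI.
; BeginPlay starts BT_AI_Boss.
; Entering the boss fight creates the W_BossEnemyHP widget and adds it to the viewport, and exiting removes and clears it.
; While the widget is valid, Tick updates its progress bar and truncated HP text from HP and HPMax.
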(event Custom|激活Boss战
  (bind _returnvalue (UserInterface|CreateWidget "/Game/UI/W_BossEnemyHP.W_BossEnemyHP_C"))
  (bind _output_get (Variables|Default|SetBossUI _returnvalue))
  (UserInterface|Viewport|AddtoViewport _output_get 0))

(event Custom|退出Boss战
  (Widget|RemovefromParent (Variables|Default|GetBossUI))
  (Variables|Default|SetBossUI 0))

(event EventBeginPlay
  (AI|RunBehaviorTree "/Game/AI/BT_AI_Boss.BT_AI_Boss"))

(event EventTick
  (params (DeltaSeconds :type Float%20%28single-precision%29))
  (bind _bossui (Variables|Default|GetBossUI)
    (:then
      (Progress|SetPercent (Variables|/Game/UI/W_BossEnemyHP.W_BossEnemyHP_C|GetPB_HP _bossui) (/ (Variables|Default|GetHP) (Variables|Default|GetHPMax)))
      (Rendering|Components|TextRender|SetText (Variables|/Game/UI/W_BossEnemyHP.W_BossEnemyHP_C|GetText__HP _bossui) (Utilities|Text|ToText(Integer) (Math|Float|Truncate (Variables|Default|GetHP)))))
    (:else)))

(fn ConstructionScript
  (|CallParentFunction))