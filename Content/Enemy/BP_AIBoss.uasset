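; BP_AIBoss is a boss enemy Blueprint that shares its health state with its AI controller.
; Every Tick it casts its controller to BP_AI控制器_Boss and copies HP and HPMax from the BPCStats component into it.
; BeginPlay and the construction script only call their parent versions, and the overlap event is disabled.
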(event EventBeginPlay
  (|CallParentFunction))

(event Collision|EventActorBeginOverlap
  (params (OtherActor :type Actor%20Object%20Reference))
  (|CallParentFunction OtherActor) ; 此节点被禁用，将不会被调用。\n从引脚连出引线来编译功能。
)

(event EventTick
  (params (DeltaSeconds :type Float%20%28single-precision%29))
  (bind _bpc_stats (Variables|Default|GetBPC_Stats))
  (|CallParentFunction DeltaSeconds)
  (bind _asbp_ai控制器_boss (Utilities|Casting|CastToBP_AI控制器_Boss (AI|GetAIController self)))
  (Variables|/Game/AI/BP_AI控制器_Boss.BP_AI控制器_Boss_C|SetHP _asbp_ai控制器_boss (Variables|/Game/基础/BPC_Stats.BPC_Stats_C|GetHP _bpc_stats))
  (Variables|/Game/AI/BP_AI控制器_Boss.BP_AI控制器_Boss_C|SetHPMax _asbp_ai控制器_boss (Variables|/Game/基础/BPC_Stats.BPC_Stats_C|GetHPMax _bpc_stats)))

(fn ConstructionScript
  (|CallParentFunction))