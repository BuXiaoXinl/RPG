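; BP_AIEnemy is a melee enemy character with AI-triggered sword combos, stealth assassination and a camera-facing investigation icon.
; Attacks play montages by combo index, buffering repeat requests for the combo continuation event.
; A timer-driven sphere trace along the blade damages "P"-tagged actors with shake, sound and blood effects.
; Damage cancels combos, plays a random reaction, launches the enemy and updates BPCStats, with death triggering ragdoll and notifying the player's quest component.
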(event Custom|连击
  ;[1 1 1] 普通攻击
  (if (Variables|Default|GetSaveATK)
    (Variables|Default|SetSaveATK false)
    (switch int (Variables|Default|Get攻击索引)
      (:0
        (CallFunction|攻击1))
      (:1
        (CallFunction|攻击2))
      (:2
        (CallFunction|攻击4)))
    (else
      (CallFunction|停止连击))))

(event Custom|停止连击
  ;[1 1 1] 普通攻击
  (Variables|Default|SetIsATK false)
  (Variables|Default|Set攻击索引 0))

(event Custom|剑轨迹
  ;[1 1 1] 普通攻击
  (bind _returnvalue (Utilities|Time|SetTimerbyEvent (delegate Custom|追踪) 0.01 true))
  (Variables|Default|Set剑轨迹定时器 _returnvalue))

(event Custom|追踪
  ;[1 1 1] 普通攻击
  (bind (_outhit _returnvalue) (Collision|SphereTraceByChannel (Transformation|GetWorldLocation (Variables|Default|Get剑尖)) (Transformation|GetWorldLocation (Variables|Default|Get剑把)) 1e+01 "TraceTypeQuery1" false 0 "None" true "(R=1.000000,G=0.000000,B=0.000000,A=1.000000)" "(R=0.000000,G=1.000000,B=0.000000,A=1.000000)" 0.1))
  (if _returnvalue
    (if (Actor|ActorHasTag (.HitActor (Collision|BreakHitResult _outhit)) "P")
      (Utilities|FlowControl|DoOnce false :!label _label
        (:Completed
          (Game|Damage|ApplyDamage (.HitActor (Collision|BreakHitResult _outhit)) -1e+01 0 0)
          (Camera|PlayWorldCameraShake "/Game/Player/BP_普攻旧版摄像机晃动.BP_普攻旧版摄像机晃动_C" (.Location (Collision|BreakHitResult _outhit)) 0.0 2e+03)
          (Audio|SpawnSoundatLocation "/Game/Music/MS_剑攻击.MS_剑攻击" (Transformation|GetActorLocation) "0, 0, 0" 1.0 1.0 0.0 "/Game/Music/SA_角色音效衰减.SA_角色音效衰减" 0)
          (Effects|SpawnEmitteratLocation "/Game/Realistic_Starter_VFX_Pack_Vol2/Particles/Blood/P_Blood_Splat_Cone.P_Blood_Splat_Cone" (.Location (Collision|BreakHitResult _outhit)) (Math|Rotator|MakeRotfromXY (.Normal (Collision|BreakHitResult _outhit)) (.Normal (Collision|BreakHitResult _outhit))) "0.400000,0.400000,0.400000" true "AutoRelease")
          (Utilities|FlowControl|Delay 0.5)
          (goto _label Reset))))))

(event Custom|停止剑轨迹追踪
  ;[1 1 1] 普通攻击
  (Utilities|Time|ClearandInvalidateTimerbyHandle (Variables|Default|Get剑轨迹定时器)))

(event Custom|攻击4
  ;[1 1 1] 普通攻击
  (Utilities|FlowControl|DoOnce false :!label _label
    (:Completed
      (Utilities|FlowControl|Delay 0.1)
      (Animation|Montage|PlayMontage (Variables|Character|GetMesh) "/Game/Player/Anim/Attack3_Montage.Attack3_Montage" (Variables|Default|Get攻击速度)
        (:then
          (Variables|Default|Set攻击索引 4)
          (goto _label Reset))))))

(event Custom|攻击1
  ;[1 1 1] 普通攻击
  (Utilities|FlowControl|DoOnce false :!label _label
    (:Completed
      (Utilities|FlowControl|Delay 0.1)
      (Animation|Montage|PlayMontage (Variables|Character|GetMesh) "/Game/Player/Anim/Attack1_Montage.Attack1_Montage" (Variables|Default|Get攻击速度)
        (:then
          (Variables|Default|Set攻击索引 1)
          (goto _label Reset))))))

(event Custom|攻击
  ;[1 1 1] 普通攻击
  (if (Variables|Default|GetIsATK)
    (Variables|Default|SetSaveATK true)
    (else
      (Variables|Default|SetIsATK true)
      (switch int (Variables|Default|Get攻击索引)
        (:0
          (CallFunction|攻击1))
        (:1
          (CallFunction|攻击2))
        (:2
          (CallFunction|攻击4))))))

(event Custom|攻击2
  ;[1 1 1] 普通攻击
  (Utilities|FlowControl|DoOnce false :!label _label
    (:Completed
      (Utilities|FlowControl|Delay 0.1)
      (Animation|Montage|PlayMontage (Variables|Character|GetMesh) "/Game/Player/Anim/Attack2_Montage.Attack2_Montage" (Variables|Default|Get攻击速度)
        (:then
          (Variables|Default|Set攻击索引 2)
          (goto _label Reset))))))

(event Custom|攻击3
  ;[1 1 1] 普通攻击
  (Utilities|FlowControl|DoOnce false :!label _label
    (:Completed
      (Utilities|FlowControl|Delay 0.1)
      (Animation|Montage|PlayMontage (Variables|Character|GetMesh) "/Game/Player/Anim/Kick_Montage.Kick_Montage" (Variables|Default|Get攻击速度)
        (:then
          (Variables|Default|Set攻击索引 3)
          (goto _label Reset))))))

(event EventBeginPlay
  (|CallParentFunction) ; 此节点被禁用，将不会被调用。\n从引脚连出引线来编译功能。
)

(event Collision|EventActorBeginOverlap
  (params (OtherActor :type Actor%20Object%20Reference)))

(event Game|Damage|EventAnyDamage
  (params (Damage :type Float%20%28single-precision%29) (DamageType :type Damage%20Type%20Object%20Reference) (InstigatedBy :type Controller%20Object%20Reference) (DamageCauser :type Actor%20Object%20Reference))
  (CallFunction|停止连击)
  (Animation|PlayAnimMontage (Utilities|Array|Get(acopy) (Variables|Default|Get受击动画) (Math|Random|RandomIntegerinRange 0 (- (Utilities|Array|Length (Variables|Default|Get受击动画)) 1))) 1.0 "None")
  (bind _asbp_third_person_character (Utilities|Casting|CastToBP_ThirdPersonCharacter (Game|GetPlayerCharacter 0)))
  (Character|LaunchCharacter (* (Math|Vector|GetForwardVector (Transformation|GetActorRotation _asbp_third_person_character)) 7e+02) false false)
  (bind _isdie (Default|UpdataHP (Variables|Default|GetBPC_Stats) Damage))
  (if _isdie
    (Rendering|SetVisibility (Variables|Default|GetHPUI) false false)
    (Collision|SetCollisionEnabled (Variables|Default|GetSphere) "NoCollision")
    (Physics|SetSimulatePhysics (Variables|Character|GetMesh) true)
    (Audio|SpawnSoundatLocation "/Game/Music/SC_Die.SC_Die" (Transformation|GetActorLocation) "0, 0, 0" 1.0 1.0 0.0 "/Game/Music/SA_角色音效衰减.SA_角色音效衰减" 0)
    (Default|消灭敌人 (Variables|/Game/ThirdPerson/Blueprints/BP_ThirdPersonCharacter.BP_ThirdPersonCharacter_C|GetBPC_任务 (CallFunction|GetPlayer)) self)
    (else
      (Audio|SpawnSoundatLocation "/Game/Music/素材/667299__pekena_larva__voc_male_land_03.667299__pekena_larva__voc_male_land_03" (Transformation|GetActorLocation) "0, 0, 0" 1.0 (Math|Random|RandomFloatinRange 1.5 1.3) 0.0 0 0))))

(event EventTick
  (params (DeltaSeconds :type Float%20%28single-precision%29))
  (|CallParentFunction DeltaSeconds)
  (Transformation|SetWorldRotation (Variables|Default|Get调查图标) (Math|Rotator|FindLookatRotation (Transformation|GetWorldLocation (Variables|Default|Get调查图标)) (Transformation|GetWorldLocation (Variables|/Script/Engine.PlayerCameraManager|GetTransformComponent (Game|GetPlayerCameraManager 0)))) false false))

(fn ConstructionScript
  (|CallParentFunction))

(fn 暗杀
  (Animation|PlayAnimMontage "/Game/Player/Anim/Paired_Knife_Stealth_KidneyAndNeck_Vic_Montage.Paired_Knife_Stealth_KidneyAndNeck_Vic_Montage" 1.0 "None")
  (CallFunction|Die)
  (Rendering|SetVisibility (Variables|Default|Get暗杀文本) false false)
  (return (Transformation|GetWorldLocation (Variables|Default|GetBeiCi)) (Transformation|GetActorRotation)))

(fn 敌人AI连击
  (if (Variables|Default|GetCanATK)
    (CallFunction|攻击)))

(fn 启用调查图标
  (Rendering|SetVisibility (Variables|Default|Get调查图标) true false))

(fn 禁用调查图标
  (Rendering|SetVisibility (Variables|Default|Get调查图标) false false))

(fn AIATK
  (CallFunction|敌人AI连击)
  (return 0.4))