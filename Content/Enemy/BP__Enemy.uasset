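; Enemy character with a floating health bar, hit reactions and an assassination prompt that shows while a "P"-tagged actor overlaps its Sphere.
; Tick turns the bar and prompt toward the player camera.
; AnyDamage plays a random hit montage, launches the enemy along the player's facing and updates BPCStats, ragdolling it on death.
; A separate Die event delays ragdoll and death sound; the 暗杀 (assassination) function returns only zero transforms.
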(event OnComponentBeginOverlap(Sphere)
  (params (OverlappedComponent :type Primitive%20Component%20Object%20Reference) (OtherActor :type Actor%20Object%20Reference) (OtherComp :type Primitive%20Component%20Object%20Reference) (OtherBodyIndex :type Integer) (bFromSweep :type Boolean) (SweepResult :type Hit%20Result%20Structure%20%28by%20ref%29))
  (if (Actor|ActorHasTag OtherActor "P")
    (Rendering|SetVisibility (Variables|Default|Get暗杀文本) true false)))

(event OnComponentEndOverlap(Sphere)
  (params (OverlappedComponent :type Primitive%20Component%20Object%20Reference) (OtherActor :type Actor%20Object%20Reference) (OtherComp :type Primitive%20Component%20Object%20Reference) (OtherBodyIndex :type Integer))
  (if (Actor|ActorHasTag OtherActor "P")
    (Rendering|SetVisibility (Variables|Default|Get暗杀文本) false false)))

(event Custom|Die
  (Utilities|FlowControl|Sequence
    (:then_0
      (Rendering|SetVisibility (Variables|Default|GetHPUI) false false)
      (Collision|SetCollisionEnabled (Variables|Default|GetSphere) "NoCollision")
      (Utilities|FlowControl|Delay 2.5)
      (Physics|SetSimulatePhysics (Variables|Character|GetMesh) true))
    (:then_1
      (Utilities|FlowControl|Delay 1.7)
      (Audio|SpawnSoundatLocation "/Game/Music/SC_Die.SC_Die" (Transformation|GetActorLocation) "0, 0, 0" 1.0 1.0 0.0 "/Game/Music/SA_角色音效衰减.SA_角色音效衰减" 0))))

(event EventBeginPlay
  (bind _asw_enemy_hp (Utilities|Casting|CastToW_EnemyHP (UserInterface|GetWidget (Variables|Default|GetHPUI))))
  (Variables|Default|SetAs%20W%20Enemy%20HP _asw_enemy_hp)
  (Default|UpdataHP (Variables|Default|GetBPC_Stats) 0.0))

(event EventTick
  (params (DeltaSeconds :type Float%20%28single-precision%29))
  (Transformation|SetWorldRotation (Variables|Default|Get暗杀文本) (Math|Rotator|FindLookatRotation (Transformation|GetWorldLocation (Variables|Default|Get暗杀文本)) (Transformation|GetWorldLocation (Variables|/Script/Engine.PlayerCameraManager|GetTransformComponent (Game|GetPlayerCameraManager 0)))) false false))

(event Game|Damage|EventAnyDamage
  (params (Damage :type Float%20%28single-precision%29) (DamageType :type Damage%20Type%20Object%20Reference) (InstigatedBy :type Controller%20Object%20Reference) (DamageCauser :type Actor%20Object%20Reference))
  (Animation|PlayAnimMontage (Utilities|Array|Get(acopy) (Variables|Default|Get受击动画) (Math|Random|RandomIntegerinRange 0 (- (Utilities|Array|Length (Variables|Default|Get受击动画)) 1))) 1.0 "None")
  (bind _asbp_third_person_character (Utilities|Casting|CastToBP_ThirdPersonCharacter (Game|GetPlayerCharacter 0)))
  (Character|LaunchCharacter (* (Math|Vector|GetForwardVector (Transformation|GetActorRotation _asbp_third_person_character)) 7e+02) false false)
  (bind _isdie (Default|UpdataHP (Variables|Default|GetBPC_Stats) Damage))
  (if _isdie
    (Rendering|SetVisibility (Variables|Default|GetHPUI) false false)
    (Collision|SetCollisionEnabled (Variables|Default|GetSphere) "NoCollision")
    (Physics|SetSimulatePhysics (Variables|Character|GetMesh) true)
    (Audio|SpawnSoundatLocation "/Game/Music/SC_Die.SC_Die" (Transformation|GetActorLocation) "0, 0, 0" 1.0 1.0 0.0 "/Game/Music/SA_角色音效衰减.SA_角色音效衰减" 0)
    (else
      (Audio|SpawnSoundatLocation "/Game/Music/素材/667299__pekena_larva__voc_male_land_03.667299__pekena_larva__voc_male_land_03" (Transformation|GetActorLocation) "0, 0, 0" 1.0 (Math|Random|RandomFloatinRange 1.5 1.3) 0.0 0 0))))

(fn ConstructionScript)

(fn 暗杀
  (return "0, 0, 0" "0, 0, 0"))