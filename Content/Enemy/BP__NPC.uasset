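; Quest-giver NPC that talks to the player and then offers a list of quests.
; A sphere overlap with "P"-tagged actors toggles a quest text label, which turns toward the camera every tick.
; Each 任务 call advances the dialogue widget, then opens the quest widget filled from 任务结构 with this NPC as giver.
; Calling it again or 关闭任务 closes that widget and restores game-only input.
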(event OnComponentBeginOverlap(Sphere)
  (params (OverlappedComponent :type Primitive%20Component%20Object%20Reference) (OtherActor :type Actor%20Object%20Reference) (OtherComp :type Primitive%20Component%20Object%20Reference) (OtherBodyIndex :type Integer) (bFromSweep :type Boolean) (SweepResult :type Hit%20Result%20Structure%20%28by%20ref%29))
  (if (Actor|ActorHasTag OtherActor "P")
    (Rendering|SetVisibility (Variables|Default|Get任务文本) true false)))

(event OnComponentEndOverlap(Sphere)
  (params (OverlappedComponent :type Primitive%20Component%20Object%20Reference) (OtherActor :type Actor%20Object%20Reference) (OtherComp :type Primitive%20Component%20Object%20Reference) (OtherBodyIndex :type Integer))
  (if (Actor|ActorHasTag OtherActor "P")
    (Rendering|SetVisibility (Variables|Default|Get任务文本) false false)))

(event Custom|关闭任务
  (bind _returnvalue (Game|GetPlayerController 0))
  (Widget|RemovefromParent (Variables|Default|Get任务界面))
  (Variables|Default|Set任务界面 0)
  (Variables|Default|Set任务界面是否激活 false)
  (Variables|/Script/Engine.PlayerController|SetbShowMouseCursor _returnvalue false)
  (Input|SetInputModeGameOnly _returnvalue false))

(event Custom|打开任务界面
  (bind _returnvalue (UserInterface|CreateWidget "/Game/UI/w_任务界面.w_任务界面_C"))
  (bind _output_get (Variables|Default|Set任务界面 _returnvalue))
  (UserInterface|Viewport|AddtoViewport _output_get 0)
  (Variables|Default|Set任务界面是否激活 true)
  (Variables|/Game/UI/w_任务界面.w_任务界面_C|Set任务发布者 (Variables|Default|Get任务界面) self)
  (for _array_element (Variables|Default|Get任务结构)
    (Default|添加任务 (Variables|Default|Get任务界面) _array_element)))

(event EventBeginPlay)

(event Event任务
  (bind _returnvalue (Game|GetPlayerController 0))
  (bind _returnvalue_2 (Game|GetPlayerController 0))
  (if (not (Variables|Default|Get任务界面是否激活))
    (if (not (Variables|Default|GetIs对话))
      (bind _returnvalue_3 (UserInterface|CreateWidget "/Game/UI/W_对话.W_对话_C"))
      (bind _output_get (Variables|Default|Set对话界面 _returnvalue_3))
      (UserInterface|Viewport|AddtoViewport _output_get 0)
      (Rendering|Components|TextRender|SetText (Variables|/Game/UI/W_对话.W_对话_C|GetText_对话 (Variables|Default|Get对话界面)) (Utilities|Text|ToText(String) (Utilities|Array|Get(acopy) (Variables|Default|Get对话) (Variables|Default|Get对话索引))))
      (Math|Integer|IncrementInt (Variables|Default|Get对话索引)
        (:%20%20
          (Variables|Default|SetIs对话 true)
          (Variables|/Script/Engine.PlayerController|SetbShowMouseCursor _returnvalue_2 true)
          (Input|SetInputModeGameandUI _returnvalue_2 (Variables|Default|Get任务界面) "DoNotLock" true false)))
      (else
        (Rendering|Components|TextRender|SetText (Variables|/Game/UI/W_对话.W_对话_C|GetText_对话 (Variables|Default|Get对话界面)) (Utilities|Text|ToText(String) (Utilities|Array|Get(acopy) (Variables|Default|Get对话) (Variables|Default|Get对话索引))))
        (Math|Integer|IncrementInt (Variables|Default|Get对话索引)
          (:%20%20
            (if (> (Variables|Default|Get对话索引) (Utilities|Array|Length (Variables|Default|Get对话)))
              (Widget|RemovefromParent (Variables|Default|Get对话界面))
              (Variables|Default|Set对话索引 0)
              (Variables|Default|SetIs对话 false)
              (CallFunction|打开任务界面))))))
    (else
      (Widget|RemovefromParent (Variables|Default|Get任务界面))
      (Variables|Default|Set任务界面 0)
      (Variables|Default|Set任务界面是否激活 false)
      (Variables|/Script/Engine.PlayerController|SetbShowMouseCursor _returnvalue false)
      (Input|SetInputModeGameOnly _returnvalue false))))

(event EventTick
  (params (DeltaSeconds :type Float%20%28single-precision%29))
  (Transformation|SetWorldRotation (Variables|Default|Get任务文本) (Math|Rotator|FindLookatRotation (Transformation|GetWorldLocation (Variables|Default|Get任务文本)) (Transformation|GetWorldLocation (Variables|/Script/Engine.PlayerCameraManager|GetTransformComponent (Game|GetPlayerCameraManager 0)))) false false))

(fn ConstructionScript)