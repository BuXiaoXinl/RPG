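; BP_动物 is an enemy animal that roams, chases the player on sight and attacks in melee.
; It moves to random reachable points with short pauses, replaying its attack sound periodically as an ambient call.
; PawnSensing sightings of "P"-tagged pawns trigger AIMoveTo toward player 0.
; Arrival plays an IsATK-guarded montage whose notify runs a forward sphere trace and applies damage on a hit.
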(event OnSeePawn(PawnSensing)
  (params (Pawn :type Pawn%20Object%20Reference))
  (bind _returnvalue (Transformation|GetActorLocation))
  (if (Actor|ActorHasTag Pawn "P")
    (AI|AIMoveTo self "0, 0, 0" (Game|GetPlayerCharacter 0) 4e+02 false
      (:OnSuccess
        (if (not (Variables|Default|GetIsATK))
          (Variables|Default|SetIsATK true)
          (Animation|Montage|PlayMontage (Variables|Character|GetMesh) (Variables|Default|Get攻击蒙太奇)
            (:then
              (Audio|SpawnSoundatLocation (Variables|Default|Get攻击音效) (Transformation|GetActorLocation) "0, 0, 0" 1.0 1.0 0.0 "/Game/Music/SA_角色音效衰减.SA_角色音效衰减" 0))
            (:OnCompleted
              (Variables|Default|SetIsATK false))
            (:OnNotifyBegin
              (bind (_outhit _returnvalue_2) (Collision|SphereTraceForObjects _returnvalue (+ _returnvalue (* (Math|Vector|GetForwardVector (Transformation|GetActorRotation)) 3.5e+02)) 1.3e+02 (Utilities|Array|MakeArray "ObjectTypeQuery3") false 0 "None"))
              (if _returnvalue_2
                (Game|Damage|ApplyDamage (.HitActor (Collision|BreakHitResult _outhit)) (Variables|Default|Get攻击伤害) 0 0)))))))))

(event Custom|动物散步
  (AI|AIMoveTo self (.RandomLocation (AI|Navigation|GetRandomReachablePointinRadius (Transformation|GetActorLocation) 5e+03 0 0)) 0 5.0 false
    (:OnSuccess
      (Utilities|FlowControl|Delay 3.0)
      (CallFunction|动物散步))))

(event EventBeginPlay
  (CallFunction|动物散步)
  (Utilities|FlowControl|Delay (Math|Random|RandomFloatinRange 15.0 2e+01) :!label _label)
  (Audio|SpawnSoundatLocation (Variables|Default|Get攻击音效) (Transformation|GetActorLocation) "0, 0, 0" 0.7 1.0 0.0 "/Game/Music/SA_角色音效衰减.SA_角色音效衰减" 0)
  (goto _label))

(fn ConstructionScript)