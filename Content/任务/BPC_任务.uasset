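; Quest component (BPC_任务) that tracks the active quest's objectives and shows them in a W_任务追踪 HUD widget created at BeginPlay.
; Events set the quest title, fill the objective list, and report killed enemies or opened chests against each objective.
; Kills shrink a working target array written back by reference into the quest struct.
; Completed objectives increment a counter that, at the objective total, clears the quest and plays the completion animation and sound.
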(event Custom|设置任务文本
  (bind _任务追踪界面 (Variables|Default|Get任务追踪界面))
  (Rendering|Components|TextRender|SetText (Variables|/Game/UI/W_任务追踪.W_任务追踪_C|GetText_当前任务 _任务追踪界面) (Utilities|Text|ToText(String) (.Name (Utilities|Struct|BreakS__任务结构 (Variables|Default|Get任务结构)))))
  (Default|显示任务追踪 _任务追踪界面))

(event Custom|追踪任务
  (Default|填充目标 (Variables|Default|Get任务追踪界面) (.任务目标 (Variables|Default|Get任务结构))))

(event Custom|消灭敌人
  (params (被消除敌人 :type Actor%20Object%20Reference))
  (for _array_element (.任务目标 (Variables|Default|Get任务结构))
    (if (and (not (.是否完成 (Utilities|Struct|BreakS_任务目标 _array_element))) (.消灭敌人目标 (Utilities|Struct|BreakS_任务目标 _array_element)))
      (if (!= (Utilities|Array|Length (Variables|Default|Get被消灭敌人数组)) 0)
        _
        (else
          (bind _output_get (Variables|Default|Set被消灭敌人数组 (.任务目标 (Utilities|Struct|BreakS_任务目标 _array_element))))))
      (Utilities|Array|RemoveItem _output_get 被消除敌人)
      (|SetBy-RefVar _array_element (Utilities|Struct|MakeS_任务目标 (.Name (Utilities|Struct|BreakS_任务目标 _array_element)) false (Variables|Default|Get被消灭敌人数组) (.任务箱子 (Utilities|Struct|BreakS_任务目标 _array_element)) (.消灭敌人目标 (Utilities|Struct|BreakS_任务目标 _array_element)) (.完成箱子目标 (Utilities|Struct|BreakS_任务目标 _array_element))))
      (if (== (Utilities|Array|Length (Variables|Default|Get被消灭敌人数组)) 0)
        (|SetBy-RefVar _array_element (Utilities|Struct|MakeS_任务目标 (.Name (Utilities|Struct|BreakS_任务目标 _array_element)) true 0 (.任务箱子 (Utilities|Struct|BreakS_任务目标 _array_element)) (.消灭敌人目标 (Utilities|Struct|BreakS_任务目标 _array_element)) (.完成箱子目标 (Utilities|Struct|BreakS_任务目标 _array_element))))
        (Default|完成目标 (Variables|Default|Get任务追踪界面) _array_element)
        (CallFunction|目标完成)))))

(event Custom|打开宝箱
  (params (宝箱 :type Actor%20Object%20Reference))
  (for _array_element (.任务目标 (Variables|Default|Get任务结构))
    (if (and (== 宝箱 (.任务箱子 (Utilities|Struct|BreakS_任务目标 _array_element))) (.完成箱子目标 (Utilities|Struct|BreakS_任务目标 _array_element)))
      (|SetBy-RefVar _array_element (Utilities|Struct|MakeS_任务目标 (.Name (Utilities|Struct|BreakS_任务目标 _array_element)) (.是否完成 (Utilities|Struct|BreakS_任务目标 _array_element)) (.任务目标 (Utilities|Struct|BreakS_任务目标 _array_element)) 0 (.消灭敌人目标 (Utilities|Struct|BreakS_任务目标 _array_element)) (.完成箱子目标 (Utilities|Struct|BreakS_任务目标 _array_element))))
      (Default|完成目标 (Variables|Default|Get任务追踪界面) _array_element)
      (CallFunction|目标完成))))

(event Custom|目标完成
  (Math|Integer|IncrementInt (Variables|Default|Get完成任务数量)
    (:%20%20
      (if (>= (Variables|Default|Get完成任务数量) (Utilities|Array|Length (.任务目标 (Variables|Default|Get任务结构))))
        (Variables|Default|Set任务结构 "")
        (Variables|Default|Set完成任务数量 0)
        (Default|播放完成动画 (Variables|Default|Get任务追踪界面))
        (Audio|PlaySound2D "/Game/Music/素材/UP1.UP1" 1.0 1.0 0.0 0 0)))))

(event EventBeginPlay
  (bind _returnvalue (UserInterface|CreateWidget "/Game/UI/W_任务追踪.W_任务追踪_C"))
  (bind _output_get (Variables|Default|Set任务追踪界面 _returnvalue))
  (UserInterface|Viewport|AddtoViewport _output_get 0)
  (Default|隐藏任务追踪 _output_get))