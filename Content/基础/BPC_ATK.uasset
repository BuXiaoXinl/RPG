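; Player combat component for BP_ThirdPersonCharacter, covering a four-hit melee combo and bow aiming.
; Attack input plays montages by combo index, buffering presses in SaveATK for 连击 to continue or reset the chain.
; A timer-looped sword sphere trace and a one-shot kick trace damage "E"-tagged actors, adding camera shake, blood and sound.
; With a bow equipped, holding left mouse shows a crosshair, switches to controller-facing rotation and disables melee.
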(event Custom|连击
  ;[1 1 1] 普通攻击连击
  (if (Variables|Default|GetSaveATK)
    (Variables|Default|SetSaveATK false)
    (switch int (Variables|Default|Get攻击索引)
      (:0
        (CallFunction|攻击1))
      (:1
        (CallFunction|攻击2))
      (:2
        (CallFunction|攻击3))
      (:3
        (CallFunction|攻击4)))
    (else
      (CallFunction|停止连击))))

(event Custom|停止连击
  ;[1 1 1] 普通攻击连击
  (Variables|Default|SetIsATK false)
  (Variables|Default|Set攻击索引 0))

(event Custom|剑轨迹
  ;[1 1 1] 剑轨迹
  (bind _returnvalue (Utilities|Time|SetTimerbyEvent (delegate Custom|追踪) 0.01 true))
  (Variables|Default|Set剑轨迹定时器 _returnvalue))

(event Custom|追踪
  (bind _as_bp_third_person_character (Variables|Default|GetAs%20BP%20Third%20Person%20Character))
  ;[1 1 1] 剑轨迹
  (bind (_outhit _returnvalue) (Collision|SphereTraceByChannel (Transformation|GetWorldLocation (Variables|/Game/ThirdPerson/Blueprints/BP_ThirdPersonCharacter.BP_ThirdPersonCharacter_C|Get剑尖 _as_bp_third_person_character)) (Transformation|GetWorldLocation (Variables|/Game/ThirdPerson/Blueprints/BP_ThirdPersonCharacter.BP_ThirdPersonCharacter_C|Get剑把 _as_bp_third_person_character)) 1e+01 "TraceTypeQuery1" false 0 "None" true "(R=1.000000,G=0.000000,B=0.000000,A=1.000000)" "(R=0.000000,G=1.000000,B=0.000000,A=1.000000)" 0.1))
  (if _returnvalue
    (if (Actor|ActorHasTag (.HitActor (Collision|BreakHitResult _outhit)) "E")
      (Utilities|FlowControl|DoOnce false :!label _label
        (:Completed
          (Game|Damage|ApplyDamage (.HitActor (Collision|BreakHitResult _outhit)) -1e+01 0 0)
          (Camera|PlayWorldCameraShake "/Game/Player/BP_普攻旧版摄像机晃动.BP_普攻旧版摄像机晃动_C" (.Location (Collision|BreakHitResult _outhit)) 0.0 2e+03)
          (CallFunction|播放剑攻击声音)
          (Effects|SpawnEmitteratLocation "/Game/Realistic_Starter_VFX_Pack_Vol2/Particles/Blood/P_Blood_Splat_Cone.P_Blood_Splat_Cone" (.Location (Collision|BreakHitResult _outhit)) (Math|Rotator|MakeRotfromXY (.Normal (Collision|BreakHitResult _outhit)) (.Normal (Collision|BreakHitResult _outhit))) "0.400000,0.400000,0.400000" true "AutoRelease")
          (Utilities|FlowControl|Delay 0.5)
          (goto _label Reset))))))

(event Custom|停止剑轨迹追踪
  ;[1 1 1] 剑轨迹
  (Utilities|Time|ClearandInvalidateTimerbyHandle (Variables|Default|Get剑轨迹定时器)))

(event Custom|球体轨迹
  (bind _as_bp_third_person_character (Variables|Default|GetAs%20BP%20Third%20Person%20Character))
  (bind _球体追踪 (Variables|/Game/ThirdPerson/Blueprints/BP_ThirdPersonCharacter.BP_ThirdPersonCharacter_C|Get球体追踪 _as_bp_third_person_character))
  (bind _returnvalue (Transformation|GetWorldLocation _球体追踪))
  ;[1 1 1] 踢击攻击
  (bind (_outhit _returnvalue_2) (Collision|SphereTraceByChannel _returnvalue _returnvalue 5e+01 "TraceTypeQuery1" false 0 "None" true "(R=1.000000,G=0.000000,B=0.000000,A=1.000000)" "(R=0.000000,G=1.000000,B=0.000000,A=1.000000)" 0.1))
  (if _returnvalue_2
    (if (Actor|ActorHasTag (.HitActor (Collision|BreakHitResult _outhit)) "E")
      (Game|Damage|ApplyDamage (.HitActor (Collision|BreakHitResult _outhit)) -1e+01 0 0)
      (Camera|PlayWorldCameraShake "/Game/Player/BP_普攻旧版摄像机晃动.BP_普攻旧版摄像机晃动_C" (.Location (Collision|BreakHitResult _outhit)) 0.0 2e+03)
      (Effects|SpawnEmitteratLocation "/Game/Realistic_Starter_VFX_Pack_Vol2/Particles/Blood/P_Blood_Splat_Cone.P_Blood_Splat_Cone" (.Location (Collision|BreakHitResult _outhit)) (Math|Rotator|MakeRotfromXY (.Normal (Collision|BreakHitResult _outhit)) (.ImpactNormal (Collision|BreakHitResult _outhit))) "0.400000,0.400000,0.400000" true "AutoRelease")
      (CallFunction|播放剑攻击声音))))

(event Custom|攻击4
  ;[1 1 1] 普通攻击连击
  (Utilities|FlowControl|DoOnce false :!label _label
    (:Completed
      (Utilities|FlowControl|Delay 0.1)
      (Animation|Montage|PlayMontage (Variables|Default|Get角色网格体) "/Game/Player/Anim/Attack3_Montage.Attack3_Montage"
        (:then
          (Variables|Default|Set攻击索引 4)
          (goto _label Reset))))))

(event Custom|攻击1
  ;[1 1 1] 普通攻击连击
  (Utilities|FlowControl|DoOnce false :!label _label
    (:Completed
      (Utilities|FlowControl|Delay 0.1)
      (Animation|Montage|PlayMontage (Variables|Default|Get角色网格体) "/Game/Player/Anim/Attack1_Montage.Attack1_Montage"
        (:then
          (Variables|Default|Set攻击索引 1)
          (goto _label Reset))))))

(event Custom|攻击
  ;[1 1 1] 普通攻击连击
  (if (Variables|Default|GetIsATK)
    (Variables|Default|SetSaveATK true)
    (else
      (Variables|Default|SetIsATK true)
      (switch int (Variables|Default|Get攻击索引)
        (:0
          (CallFunction|攻击1))
        (:1
          (CallFunction|攻击2))
        (:2
          (CallFunction|攻击3))
        (:3
          (CallFunction|攻击4))))))

(event Custom|攻击2
  ;[1 1 1] 普通攻击连击
  (Utilities|FlowControl|DoOnce false :!label _label
    (:Completed
      (Utilities|FlowControl|Delay 0.1)
      (Animation|Montage|PlayMontage (Variables|Default|Get角色网格体) "/Game/Player/Anim/Attack2_Montage.Attack2_Montage"
        (:then
          (Variables|Default|Set攻击索引 2)
          (goto _label Reset))))))

(event Custom|攻击3
  ;[1 1 1] 普通攻击连击
  (Utilities|FlowControl|DoOnce false :!label _label
    (:Completed
      (Utilities|FlowControl|Delay 0.1)
      (Animation|Montage|PlayMontage (Variables|Default|Get角色网格体) "/Game/Player/Anim/Kick_Montage.Kick_Montage"
        (:then
          (Variables|Default|Set攻击索引 3)
          (goto _label Reset))))))

(event Input|EnhancedActionEvents|EnhancedInputActionIA_LMouse
  (params (ActionValue :type Boolean) (ElapsedSeconds :type Float%20%28double-precision%29) (TriggeredSeconds :type Float%20%28double-precision%29) (InputAction :type Input%20Action%20Object%20Reference :default "/Game/ThirdPerson/Input/Actions/IA_LMouse.IA_LMouse"))
  (bind _as_bp_third_person_character (Variables|Default|GetAs%20BP%20Third%20Person%20Character))
  (bind _as_bp_third_person_character_2 (Variables|Default|GetAs%20BP%20Third%20Person%20Character))
  (bind _charactermovement (Variables|/Script/Engine.Character|GetCharacterMovement _as_bp_third_person_character_2))
  (bind _charactermovement_2 (Variables|/Script/Engine.Character|GetCharacterMovement _as_bp_third_person_character))
  ;[1 1 1] 弓箭
  (:Started
    (if (Variables|Default|Get是否装备弓)
      (Variables|Default|SetCanATK false)
      (Variables|Default|Set射击中 true)
      (Default|手持弓 _as_bp_third_person_character)
      (Variables|/Script/Engine.CharacterMovementComponent|SetbUseControllerDesiredRotation _charactermovement_2 true)
      (Variables|/Script/Engine.CharacterMovementComponent|SetbOrientRotationToMovement _charactermovement_2 false)
      (bind _returnvalue (UserInterface|CreateWidget "/Game/UI/W_准星.W_准星_C"))
      (bind _output_get (Variables|Default|Set准星 _returnvalue))
      (UserInterface|Viewport|AddtoViewport _output_get 0)))
  (:Completed
    (if (Variables|Default|Get是否装备弓)
      (Variables|Default|SetCanATK false)
      (Variables|Default|Set射击中 false)
      (Default|手持弓 _as_bp_third_person_character_2)
      (Variables|/Script/Engine.CharacterMovementComponent|SetbUseControllerDesiredRotation _charactermovement false)
      (Variables|/Script/Engine.CharacterMovementComponent|SetbOrientRotationToMovement _charactermovement true)
      (Utilities|FlowControl|Delay 0.2)
      (bind _准星 (Variables|Default|Get准星)
        (:then
          (Widget|RemovefromParent _准星)
          (Variables|Default|Set准星 0))
        (:else)))))

(event Input|EnhancedActionEvents|EnhancedInputActionIA_ATK
  (params (ActionValue :type Boolean) (ElapsedSeconds :type Float%20%28double-precision%29) (TriggeredSeconds :type Float%20%28double-precision%29) (InputAction :type Input%20Action%20Object%20Reference :default "/Game/ThirdPerson/Input/Actions/IA_ATK.IA_ATK"))
  ;[1 1 1] 普通攻击连击
  (:Started
    (if (Variables|Default|GetCanATK)
      (CallFunction|攻击))))

(event EventBeginPlay
  ;[1 1 1] 普通攻击连击
  (bind _asbp_third_person_character (Utilities|Casting|CastToBP_ThirdPersonCharacter (Components|GetOwner)))
  (bind _output_get (Variables|Default|SetAs%20BP%20Third%20Person%20Character _asbp_third_person_character))
  (Variables|Default|Set角色网格体 (Variables|/Script/Engine.Character|GetMesh _output_get)))

(event Input|KeyboardEvents|DebugKeyQ
  (params (Key :type Key%20Structure :default "None") (ActionValue :type Input%20Action%20Value%20Structure))
  (:Pressed
    (Default|卸下手持弓 (Variables|Default|GetAs%20BP%20Third%20Person%20Character))))

(fn 播放剑攻击声音
  (Audio|SpawnSoundatLocation "/Game/Music/MS_剑攻击.MS_剑攻击" (Transformation|GetActorLocation (Components|GetOwner)) "0, 0, 0" 1.0 1.0 0.0 "/Game/Music/SA_角色音效衰减.SA_角色音效衰减" 0))