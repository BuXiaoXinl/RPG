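; Actor component that holds HP, SP, XP and level stats for the player character or an enemy.
; On BeginPlay it caches its owner and, for the player, can start a looping timer that regenerates SP until full.
; Update functions change values and push them straight to the player HUD, or to the enemy widget for HP.
; XP gain recursively carries overflow into level-ups, raising the requirement linearly and playing sounds.
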(event Custom|恢复SP
  (if (Variables|Default|Get是否恢复SP)
    (bind _ismaxsp (CallFunction|UpdataSP 0.2))
    (if _ismaxsp
      (Variables|Default|Set是否恢复SP false))))

(event EventBeginPlay
  (bind _asbp_third_person_character (Utilities|Casting|CastToBP_ThirdPersonCharacter (Components|GetOwner))
    (:then
      (Variables|Default|SetAs%20BP%20Third%20Person%20Character _asbp_third_person_character)
      (if (Variables|Default|Get是否恢复SP定时器)
        (Utilities|Time|SetTimerbyEvent (delegate Custom|恢复SP) 0.2 true)))
    (:CastFailed
      (bind _asbp__enemy (Utilities|Casting|CastToBP__Enemy (Components|GetOwner)))
      (Variables|Default|SetAs%20BP%20%20Enemy _asbp__enemy))))

(fn UpdataHP
  (params (UpdataHP :type Float%20%28double-precision%29))
  (Variables|Default|SetHP (Math|Float|Clamp(Float) (+ (Variables|Default|GetHP) UpdataHP) 0.0 (Variables|Default|GetHPMax)))
  (Progress|SetPercent (select (Variables|Default|GetIsPlayer) (Variables|/Game/UI/W_PlayerHUD.W_PlayerHUD_C|GetPB_HP (Variables|/Game/ThirdPerson/Blueprints/BP_ThirdPersonCharacter.BP_ThirdPersonCharacter_C|GetPlayerHUD (Variables|Default|GetAs%20BP%20Third%20Person%20Character))) (Variables|/Game/UI/W_EnemyHP.W_EnemyHP_C|GetPB_HP (Variables|/Game/Enemy/BP__Enemy.BP__Enemy_C|GetAs%20W%20Enemy%20HP (Variables|Default|GetAs%20BP%20%20Enemy)))) (/ (Variables|Default|GetHP) (Variables|Default|GetHPMax)))
  (Rendering|Components|TextRender|SetText (select (Variables|Default|GetIsPlayer) (Variables|/Game/UI/W_PlayerHUD.W_PlayerHUD_C|GetText_HP (Variables|/Game/ThirdPerson/Blueprints/BP_ThirdPersonCharacter.BP_ThirdPersonCharacter_C|GetPlayerHUD (Variables|Default|GetAs%20BP%20Third%20Person%20Character))) (Variables|/Game/UI/W_EnemyHP.W_EnemyHP_C|GetText__HP (Variables|/Game/Enemy/BP__Enemy.BP__Enemy_C|GetAs%20W%20Enemy%20HP (Variables|Default|GetAs%20BP%20%20Enemy)))) (Utilities|Text|ToText(Float) (Variables|Default|GetHP) "HalfToEven"))
  (return (== (Variables|Default|GetHP) 0.0)))

(fn UpdataHPMax
  (params (UpdataHPMax :type Float%20%28double-precision%29))
  (bind _as_bp_third_person_character (Variables|Default|GetAs%20BP%20Third%20Person%20Character))
  (bind _playerhud (Variables|/Game/ThirdPerson/Blueprints/BP_ThirdPersonCharacter.BP_ThirdPersonCharacter_C|GetPlayerHUD _as_bp_third_person_character))
  (bind _output_get (Variables|Default|SetHPMax (+ (Variables|Default|GetHPMax) UpdataHPMax)))
  (Variables|Default|SetHP _output_get)
  (Progress|SetPercent (Variables|/Game/UI/W_PlayerHUD.W_PlayerHUD_C|GetPB_HP _playerhud) (/ (Variables|Default|GetHP) (Variables|Default|GetHPMax)))
  (Rendering|Components|TextRender|SetText (Variables|/Game/UI/W_PlayerHUD.W_PlayerHUD_C|GetText_HP _playerhud) (Utilities|Text|ToText(Float) (Variables|Default|GetHP) "HalfToEven")))

(fn UpdataSP
  (params (UpdataSP :type Float%20%28double-precision%29))
  (Variables|Default|SetSP (Math|Float|Clamp(Float) (+ (Variables|Default|GetSP) UpdataSP) 0.0 (Variables|Default|GetSPMax)))
  (Progress|SetPercent (Variables|/Game/UI/W_PlayerHUD.W_PlayerHUD_C|GetPB_SP (Variables|/Game/ThirdPerson/Blueprints/BP_ThirdPersonCharacter.BP_ThirdPersonCharacter_C|GetPlayerHUD (Variables|Default|GetAs%20BP%20Third%20Person%20Character))) (/ (Variables|Default|GetSP) (Variables|Default|GetSPMax)))
  (return (== (Variables|Default|GetSP) 0.0) (== (Variables|Default|GetSP) (Variables|Default|GetSPMax))))

(fn UpdataSPMax
  (params (UpdataSPMax :type Float%20%28double-precision%29))
  (bind _output_get (Variables|Default|SetSPMax (+ (Variables|Default|GetSPMax) UpdataSPMax)))
  (Variables|Default|SetSP _output_get)
  (Progress|SetPercent (Variables|/Game/UI/W_PlayerHUD.W_PlayerHUD_C|GetPB_SP (Variables|/Game/ThirdPerson/Blueprints/BP_ThirdPersonCharacter.BP_ThirdPersonCharacter_C|GetPlayerHUD (Variables|Default|GetAs%20BP%20Third%20Person%20Character))) (/ (Variables|Default|GetSP) (Variables|Default|GetSPMax))))

(fn UpdataXP
  (params (UpdataSP :type Float%20%28double-precision%29))
  (bind _as_bp_third_person_character (Variables|Default|GetAs%20BP%20Third%20Person%20Character))
  (bind _playerhud (Variables|/Game/ThirdPerson/Blueprints/BP_ThirdPersonCharacter.BP_ThirdPersonCharacter_C|GetPlayerHUD _as_bp_third_person_character))
  (Variables|Default|SetXP (+ (Variables|Default|GetXP) UpdataSP))
  (if (>= (Variables|Default|GetXP) (Variables|Default|GetXPMax))
    (LocalVariables|Set溢出经验值 (- (Variables|Default|GetXP) (Variables|Default|GetXPMax)))
    (Math|Integer|IncrementInt (Variables|Default|GetLV)
      (:%20%20
        (Rendering|Components|TextRender|SetText (Variables|/Game/UI/W_PlayerHUD.W_PlayerHUD_C|GetText_LV (Variables|/Game/ThirdPerson/Blueprints/BP_ThirdPersonCharacter.BP_ThirdPersonCharacter_C|GetPlayerHUD (Variables|Default|GetAs%20BP%20Third%20Person%20Character))) (Utilities|Text|ToText(Integer) (Variables|Default|GetLV)))
        (Variables|Default|SetXP 0.0)
        (CallFunction|计算升级所需经验值)
        (CallFunction|UpdataXP (LocalVariables|Get溢出经验值))
        (Audio|PlaySound2D "/Game/Music/素材/UP1.UP1" 1.0 1.0 0.0 0 0)
        (Audio|PlaySound2D "/Game/Music/素材/UP2.UP2" 1.0 1.0 0.0 0 0)))
    (else
      (Rendering|Components|TextRender|SetText (Variables|/Game/UI/W_PlayerHUD.W_PlayerHUD_C|GetText_XP _playerhud) (Utilities|Text|FormatText "{XP}/{XPMax}" (Variables|Default|GetXP) (Variables|Default|GetXPMax)))
      (Progress|SetPercent (Variables|/Game/UI/W_PlayerHUD.W_PlayerHUD_C|GetPB_XP _playerhud) (/ (Variables|Default|GetXP) (Variables|Default|GetXPMax))))))

(fn 计算升级所需经验值
  (Variables|Default|SetXPMax (+ (Variables|Default|GetXPMax) 1.5e+02)))

(fn 初始化玩家UI
  (bind _as_bp_third_person_character (Variables|Default|GetAs%20BP%20Third%20Person%20Character))
  (bind _playerhud (Variables|/Game/ThirdPerson/Blueprints/BP_ThirdPersonCharacter.BP_ThirdPersonCharacter_C|GetPlayerHUD _as_bp_third_person_character))
  (Progress|SetPercent (Variables|/Game/UI/W_PlayerHUD.W_PlayerHUD_C|GetPB_HP _playerhud) (/ (Variables|Default|GetHP) (Variables|Default|GetHPMax)))
  (Rendering|Components|TextRender|SetText (Variables|/Game/UI/W_PlayerHUD.W_PlayerHUD_C|GetText_HP _playerhud) (Utilities|Text|ToText(Float) (Variables|Default|GetHP) "HalfToEven"))
  (Progress|SetPercent (Variables|/Game/UI/W_PlayerHUD.W_PlayerHUD_C|GetPB_SP _playerhud) (/ (Variables|Default|GetSP) (Variables|Default|GetSPMax)))
  (Progress|SetPercent (Variables|/Game/UI/W_PlayerHUD.W_PlayerHUD_C|GetPB_XP _playerhud) (/ (Variables|Default|GetXP) (Variables|Default|GetXPMax)))
  (Rendering|Components|TextRender|SetText (Variables|/Game/UI/W_PlayerHUD.W_PlayerHUD_C|GetText_XP _playerhud) (Utilities|Text|FormatText "{XP}/{XPMax}" (Variables|Default|GetXP) (Variables|Default|GetXPMax)))
  (Rendering|Components|TextRender|SetText (Variables|/Game/UI/W_PlayerHUD.W_PlayerHUD_C|GetText_LV _playerhud) (Utilities|Text|ToText(Integer) (Variables|Default|GetLV))))