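; BPC_装备 is an equipment component on BP_ThirdPersonCharacter that lets the player pick up BP_装备 item actors in the world.
; On BeginPlay it caches the owner's FollowCamera.
; When IA_E starts, a short-radius sphere trace runs forward from that camera against WorldDynamic objects.
; A hit BP_装备 passes its ItemData to 添加武器, which appends it to the 装备插槽 slots, and the actor is destroyed.
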(event Input|EnhancedActionEvents|EnhancedInputActionIA_E
  (params (ActionValue :type Boolean) (ElapsedSeconds :type Float%20%28double-precision%29) (TriggeredSeconds :type Float%20%28double-precision%29) (InputAction :type Input%20Action%20Object%20Reference :default "/Game/ThirdPerson/Input/Actions/IA_E.IA_E"))
  (bind _follow_camera (Variables|Default|GetFollow%20Camera))
  (bind _returnvalue (Transformation|GetWorldLocation _follow_camera))
  (:Started
    (bind (_outhit _returnvalue_2) (Collision|SphereTraceForObjects _returnvalue (+ _returnvalue (* (Math|Vector|GetForwardVector (Transformation|GetWorldRotation _follow_camera)) 1e+03)) 15.0 (Utilities|Array|MakeArray "ObjectTypeQuery2") false 0 "None"))
    (if _returnvalue_2
      (bind _asbp_装备 (Utilities|Casting|CastToBP_装备 (.HitActor (Collision|BreakHitResult _outhit))))
      (CallFunction|添加武器 (Variables|/Game/装备/BP_装备.BP_装备_C|GetItemData _asbp_装备))
      (Actor|DestroyActor _asbp_装备))))

(event EventBeginPlay
  (bind _asbp_third_person_character (Utilities|Casting|CastToBP_ThirdPersonCharacter (Components|GetOwner)))
  (Variables|Default|SetFollow%20Camera (Variables|/Game/ThirdPerson/Blueprints/BP_ThirdPersonCharacter.BP_ThirdPersonCharacter_C|GetFollowCamera _asbp_third_person_character)))

(fn 添加武器
  (params (NewItem :type S%20插槽%20Structure%20%28by%20ref%29))
  (Utilities|Array|Add (Variables|Default|Get装备插槽) NewItem))